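; MapGenerator builds a rectangular 2D tile map of Paper2D sprites in its construction script.
; GenerateMap sizes a flattened Grid array from MaxX and MaxY, and SelectTileType marks border cells 1 and interior cells 0.
; GenerateTiles converts each index back to X/Y and adds a rotated sprite component at TileSize spacing, branching on tile type.
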(event `self.ReceiveBeginPlay`)

(event `self.ReceiveActorBeginOverlap`
  (params (OtherActor :type "Actor Object Reference")))

(event `self.ReceiveTick`
  (params (DeltaSeconds :type "Float (single-precision)")))

(fn `1Dto2D`
  (params (ArrayPosition :type Integer :default 0))
  (returns (X :type Integer) (Y :type Integer))
  (bind _maxx (`self.MaxX`))
  (return (/ ArrayPosition _maxx) (mod ArrayPosition _maxx)))

(fn `2Dto1D`
  (params (X :type Integer :default 0) (Y :type Integer :default 0))
  (returns (ArrayPosition :type Integer))
  (return (+ (* X (`self.MaxX`)) Y)))

(fn `GenerateMap`
  (`KismetArrayLibrary.Array_Resize` (`self.Grid`) (* (`self.MaxX`) (`self.MaxY`)))
  (for (_ _array_index) (`self.Grid`)
    (bind _tiletype (`self.SelectTileType` _array_index))
    (`KismetArrayLibrary.Array_Set` (`self.Grid`) _array_index _tiletype)))

(fn `GenerateTiles`
  (params (Map :type "Array of Integer"))
  (for (_array_element _array_index) Map
    (set `self.TileType` _array_element)
    (bind (_x _y) (`self.1Dto2D` _array_index))
    (if (== (`self.TileType`) 0)
      (bind _returnvalue (`KismetMathLibrary.MakeTransform` (`KismetMathLibrary.MakeVector` (`KismetMathLibrary.Conv_IntToDouble` (* _x (`self.TileSize`))) (`KismetMathLibrary.Conv_IntToDouble` (* _y (`self.TileSize`)))) (struct :`Roll` 90.0)))
      (`AddComponent|PaperSpriteComponent_3` :`RelativeTransform` _returnvalue)
      (else
        (`AddComponent|PaperSpriteComponent_2` :`RelativeTransform` _returnvalue)))))

(fn `SelectTileType`
  (params (`1DIndex` :type Integer :default 0))
  (returns (TileType :type Integer))
  (bind (_x _y) (`self.1Dto2D` `1DIndex`))
  (set `self.XPosition` _x)
  (set `self.YPosition` _y)
  (return (select `bool` (or (or (== (`self.XPosition`) 0) (== (`self.YPosition`) 0)) (or (== (`self.XPosition`) (- (`self.MaxX`) 1)) (== (`self.YPosition`) (- (`self.MaxY`) 1)))) :`true` 1)))

(fn `UserConstructionScript`
  (`self.GenerateMap`)
  (`self.GenerateTiles` (`self.Grid`)))